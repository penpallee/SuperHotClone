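; Melee enemy that roams the level at random, then chases the player and plays an attack montage on reaching them.
; Roaming chains AI moves to random reachable points; PawnSensing sightings trigger the chase, with a flag blocking new attacks until the montage ends.
; Its Destroy function activates Niagara, spawns a snow effect and starts a looping timer that lowers a global material parameter collection level before destroying the actor.
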(event OnSeePawn(PawnSensing)
  (params (Pawn :type Pawn%20Object%20Reference))
  (Utilities|FlowControl|Sequence
    (:then_0
      (Variables|Default|SetIsSeeingPlayer true)
      (CallFunction|FollowPlayer))
    (:then_1
      (Utilities|FlowControl|RetriggerableDelay 1.0))))

(event Custom|FollowPlayer
  (Variables|Default|SetCanAttack true)
  (if (Variables|Default|GetIsSeeingPlayer)
    (AI|AIMoveTo self "0, 0, 0" (Game|GetPlayerCharacter 0) 7e+01 false
      (:OnSuccess
        (if (Variables|Default|GetCanAttack)
          (Variables|Default|SetCanAttack false)
          (bind _returnvalue (Animation|PlayAnimMontage "/Game/HS_Content/Anim/SK_Mannequin_Montage_2.SK_Mannequin_Montage_2" 1.0 "None"))
          (Utilities|FlowControl|Delay _returnvalue)
          (Variables|Default|SetCanAttack true))))))

(event Custom|RandomRoam
  (AI|AIMoveTo self (.RandomLocation (AI|Navigation|GetRandomReachablePointinRadius (Transformation|GetActorLocation) 2.5e+03 0 0)) 0 5.0 false
    (:OnSuccess
      (CallFunction|RandomRoam))))

(event EventBeginPlay
  (CallFunction|RandomRoam))

(event Collision|EventActorBeginOverlap
  (params (OtherActor :type Actor%20Object%20Reference)))

(event EventTick
  (params (DeltaSeconds :type Float%20%28single-precision%29))
  (if (Variables|Default|GetIsSeeingPlayer)
    _))

(fn ConstructionScript)

(fn Destroy
  (Components|Activation|Activate (Variables|Default|GetNiagara) false)
  (Niagara|SpawnSystematLocation "/Game/HS_Content/FX/FX1_Snow.FX1_Snow" (Transformation|GetActorLocation))
  (Utilities|Time|SetTimerbyFunctionName 0 "DeathMaterial" 0.02 true))

(fn DeathMaterial
  (bind _output_get (Variables|Default|SetMaterialLevel (- (Variables|Default|GetMaterialLevel) 1.0)))
  (Rendering|Material|SetScalarParameterValue "/Game/HS_Content/Anim/MP_Gloval_snow1.MP_Gloval_snow1" "Level" _output_get :!class /Script/Engine.KismetMaterialLibrary)
  (if (<= (Variables|Default|GetMaterialLevel) 0.0)
    (CallFunction|ReturnZero)))

(fn ReturnZero
  (bind _output_get (Variables|Default|SetMaterialLevel (- (Variables|Default|GetMaterialLevel) 1.0)))
  (Rendering|Material|SetScalarParameterValue "/Game/HS_Content/Anim/MP_Gloval_snow1.MP_Gloval_snow1" "Level" _output_get :!class /Script/Engine.KismetMaterialLibrary)
  (Actor|DestroyActor))