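; Enemy character that roams at random, pursues the player once seen and attacks with a weapon spawned on its hand socket.
; Pawn sensing starts the follow logic, also run each Tick: AI MoveTo until within range, then gradual turning until nearly facing the player.
; It then snaps round and plays a pistol montage, gated by CanShoot.
; DestroyEnemy2 spawns sparkle Niagara and loops a timer that stops the enemy and lowers a dissolve-style material parameter.
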(event OnSeePawn(PawnSensing)
  (params (Pawn :type Pawn%20Object%20Reference))
  (Utilities|FlowControl|Sequence
    (:then_0
      (Variables|Default|SetIsSeeningPlayer true)
      (CallFunction|FollowPlayer))
    (:then_1
      (Utilities|FlowControl|RetriggerableDelay 1.0))))

(event Custom|FollowPlayer
  (bind _returnvalue (Transformation|GetActorUpVector))
  (bind _returnvalue_2 (Game|GetPlayerCharacter 0))
  (bind _returnvalue_3 (Transformation|GetActorLocation))
  (bind _returnvalue_4 (Transformation|GetActorLocation _returnvalue_2))
  (bind _returnvalue_5 (- _returnvalue_4 _returnvalue_3))
  (bind _returnvalue_6 (Math|Vector|Normalize _returnvalue_5))
  (bind _returnvalue_7 (Math|Rotator|MakeRotfromXZ _returnvalue_6 _returnvalue))
  ;[1 1 1] 이미 총쏘고 있는 중이 아닐 때만 처리한다
  (if (Variables|Default|GetCanShoot)
    (if (Variables|Default|GetIsSeeningPlayer)
      (if (> (Transformation|GetDistanceTo (Game|GetPlayerCharacter 0)) (Variables|Default|GetMinDistance))
        ;[1 1 1] 따라가기
        (AI|AIMoveTo self "0, 0, 0" (Game|GetPlayerCharacter 0) (Variables|Default|GetMinDistance) false)
        (else
          ;[1 1 1] 대상의 방향 차이 확인
          (if (<= (Class|KismetMathLibrary|DegAcos (Class|Actor|GetDotProductto (Game|GetPlayerCharacter 0))) 1e+01)
            ;[1 1 1] 플레이어 방향으로 몸 회전
            ;;[1 1 1] 바로 회전하고 총 쏜다
            (Transformation|SetActorRotation _returnvalue_7)
            ;[1 1 1] 총쏘기
            (Variables|Default|SetCanShoot false)
            (bind _returnvalue_8 (Animation|PlayAnimMontage "/Game/HS_Content/Anim/AM_Pistol_org.AM_Pistol_org" 1.0 "None"))
            ;[1 1 1] 애니메이션이 끝나면 총쏘기 상태 초기화
            (Utilities|FlowControl|Delay _returnvalue_8)
            (Variables|Default|SetCanShoot true)
            (Components|Animation|SetAnimationMode (Variables|Character|GetMesh) "AnimationBlueprint")
            (else
              ;;[1 1 1] 충분한 각도가 될 때까지 서서히 회전만 반복한다.
              (Transformation|SetActorRotation (Math|Interpolation|RInterpTo (Transformation|GetActorRotation) _returnvalue_7 (Utilities|Time|GetWorldDeltaSeconds) (Variables|Default|GetInterp%20Speed))))))))))

(event Custom|SpawnWeapon
  (bind _returnvalue (Game|SpawnActorfromClass (Variables|Default|GetCurrentWeapon) (Transformation|GetSocketTransform (Variables|Character|GetMesh) "WeaponSocket" "RTS_World") "Undefined" 0 0))
  (Variables|Default|SetCurrentWeaponActor _returnvalue)
  (Transformation|AttachComponentToComponent (Variables|Default|GetCurrentWeaponActor) (Variables|Character|GetMesh) "WeaponSocket" "SnapToTarget" "SnapToTarget" "SnapToTarget" true))

(event Custom|Fire)

(event Custom|Randomroam
  (AI|AIMoveTo self (.RandomLocation (AI|Navigation|GetRandomReachablePointinRadius (Transformation|GetActorLocation) 2.5e+03 0 0)) 0 5.0 false
    (:OnSuccess
      (CallFunction|Randomroam))))

(event Custom|TryDeath
  (Class|NavMovementComponent|StopActiveMovement (Variables|Character|GetCharacterMovement))
  ;[1 1 1] 따라가기
  (Variables|Default|SetblsDead true))

(event EventBeginPlay
  (CallFunction|Randomroam)
  (CallFunction|SpawnWeapon))

(event EventTick
  (params (DeltaSeconds :type Float%20%28single-precision%29))
  (if (not (Variables|Default|GetblsDead))
    (CallFunction|FollowPlayer)))

(fn ConstructionScript)

(fn DestroyEnemy2
  (Components|Activation|Activate (Variables|Default|GetNiagara) false)
  (Niagara|SpawnSystematLocation "/Game/HS_Content/FX/FX3_Sparkle.FX3_Sparkle" (Transformation|GetActorLocation))
  (Utilities|Time|SetTimerbyFunctionName 0 "DeathMaterial_sparkle" 0.01 true))

(fn DeathMaterialSparkle
  (CallFunction|TryDeath)
  (bind _output_get (Variables|Default|SetMeterialLevel (- (Variables|Default|GetMeterialLevel) 1.0)))
  (Rendering|Material|SetScalarParameterValueonMaterials (Variables|Character|GetMesh) "level_sparkle" _output_get)
  (if (<= (Variables|Default|GetMeterialLevel) 0.0)
    _))

(fn ReturnZero
  (bind _output_get (Variables|Default|SetMeterialLevel (- (Variables|Default|GetMeterialLevel) 1.0)))
  (Rendering|Material|SetScalarParameterValue "/Game/HS_Content/Anim/MP_Gloval1.MP_Gloval1" "Level" _output_get :!class /Script/Engine.KismetMaterialLibrary))