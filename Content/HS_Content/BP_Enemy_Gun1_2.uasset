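; Gun-wielding enemy that roams randomly until pawn sensing spots a pawn, then pursues and shoots the player.
; Tick drives FollowPlayer, which closes to minimum range, turns smoothly until roughly facing, then snaps, spawns a BP_Bullet and waits out a cooldown.
; A weapon actor attaches to the hand socket at BeginPlay.
; Any bullet overlap kills it, triggering sparkle effects and a timer-driven Material Parameter Collection fade before destruction.
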(event OnSeePawn(PawnSensing)
  (params (Pawn :type Pawn%20Object%20Reference))
  (Utilities|FlowControl|Sequence
    (:then_0
      (Variables|Default|SetIsSeeningPlayer true)
      (CallFunction|FollowPlayer))
    (:then_1
      (Utilities|FlowControl|RetriggerableDelay 1.0))))

(event Custom|FollowPlayer
  (bind _returnvalue (Transformation|GetActorUpVector))
  (bind _returnvalue_2 (Game|GetPlayerCharacter 0))
  (bind _returnvalue_3 (Transformation|GetActorLocation))
  (bind _returnvalue_4 (Transformation|GetActorLocation _returnvalue_2))
  (bind _returnvalue_5 (- _returnvalue_4 _returnvalue_3))
  (bind _returnvalue_6 (Math|Vector|Normalize _returnvalue_5))
  (bind _returnvalue_7 (Math|Rotator|MakeRotfromXZ _returnvalue_6 _returnvalue))
  ;[1 1 1] 이미 총쏘고 있는 중이 아닐 때만 처리한다
  (if (Variables|Default|GetCanShoot)
    (if (Variables|Default|GetIsSeeningPlayer)
      (if (> (Transformation|GetDistanceTo (Game|GetPlayerCharacter 0)) (Variables|Default|GetMinDistance))
        ;[1 1 1] 따라가기
        (AI|AIMoveTo self "0, 0, 0" (Game|GetPlayerCharacter 0) (Variables|Default|GetMinDistance) false)
        (else
          ;[1 1 1] 대상의 방향 차이 확인
          (if (<= (Class|KismetMathLibrary|DegAcos (Class|Actor|GetDotProductto (Game|GetPlayerCharacter 0))) 1e+01)
            ;[1 1 1] 플레이어 방향으로 몸 회전
            ;;[1 1 1] 바로 회전하고 총 쏜다
            (Transformation|SetActorRotation _returnvalue_7)
            (Variables|Default|SetCanShoot false)
            (Animation|PlayAnimMontage "/Game/HS_Content/Anim/Enemy_gun_org2.Enemy_gun_org2" 0.0 "None")
            (Game|SpawnActorfromClass "/Game/Blueprints/BP_Bullet.BP_Bullet_C" (Transformation|GetWorldTransform (Variables|Default|GetScene)) "Undefined" 0 0)
            ;[1 1 1] 애니메이션이 끝난 후!!!!  1.총쏘기 상태 초기화 2. 애니모드 초기화
            (Utilities|FlowControl|Delay 6.0)
            (Variables|Default|SetCanShoot true)
            (Components|Animation|SetAnimationMode (Variables|Character|GetMesh) "AnimationBlueprint")
            (else
              ;;[1 1 1] 충분한 각도가 될 때까지 서서히 회전만 반복한다.
              (Transformation|SetActorRotation (Math|Interpolation|RInterpTo (Transformation|GetActorRotation) _returnvalue_7 (Utilities|Time|GetWorldDeltaSeconds) (Variables|Default|GetInterp%20Speed))))))))))

(event Custom|SpawnWeapon
  ;[1 1 1] Gun
  (bind _returnvalue (Game|SpawnActorfromClass (Variables|Default|GetCurrentWeapon) (Math|Transform|MakeTransform "0, 0, 0") "Undefined" 0 0))
  (Variables|Default|SetCurrentWeaponActor _returnvalue)
  (Transformation|AttachComponentToComponent (Variables|Default|GetCurrentWeaponActor) (Variables|Character|GetMesh) "hand_rSocket" "KeepRelative" "KeepRelative" "KeepRelative" true))

(event Custom|Fire
  (bind _playerref (Variables|Default|GetPlayerRef))
  (bind _mesh (Variables|Character|GetMesh))
  (bind _returnvalue (Transformation|GetWorldLocation _mesh))
  (bind _returnvalue_2 (Transformation|GetActorLocation _playerref))
  (bind _returnvalue_3 (Math|Rotator|FindLookatRotation _returnvalue _returnvalue_2))
  ;[1 1 1] Gun
  (Game|SpawnActorfromClass "/Game/Blueprints/BP_Bullet.BP_Bullet_C" (Math|Transform|MakeTransform "0, 0, 0" (Math|Rotator|MakeRotator (.roll _returnvalue_3) 0.0 (.yaw _returnvalue_3)) "1.000000,1.000000,1.000000") "AlwaysSpawn" 0 0)
  (Utilities|FlowControl|Delay (Variables|Default|GetTimeBetoweenShots))
  (CallFunction|Fire))

(event Custom|Randomroam
  (if (Variables|Default|GetCanShoot)
    (AI|AIMoveTo self (.RandomLocation (AI|Navigation|GetRandomReachablePointinRadius (Transformation|GetActorLocation) 2.5e+03 0 0)) 0 5.0 false
      (:OnSuccess
        (CallFunction|Randomroam)))))

(event Custom|TryDeath
  (Class|NavMovementComponent|StopActiveMovement (Variables|Character|GetCharacterMovement))
  (Variables|Default|SetblsDead true)
  (CallFunction|DestroyEnemy2))

(event Collision|EventActorBeginOverlap
  (params (OtherActor :type Actor%20Object%20Reference))
  (Utilities|Casting|CastToBP_Bullet OtherActor)
  (CallFunction|TryDeath))

(event EventBeginPlay
  (CallFunction|SpawnWeapon)
  (CallFunction|Randomroam))

(event EventTick
  (params (DeltaSeconds :type Float%20%28single-precision%29))
  (if (not (Variables|Default|GetblsDead))
    (CallFunction|FollowPlayer)))

(fn ConstructionScript
  (Transformation|AttachComponentToComponent (Variables|Character|GetMesh) 0 "None" "KeepRelative" "KeepRelative" "KeepRelative" true))

(fn DestroyEnemy2
  (Components|Activation|Activate (Variables|Default|GetNiagara) false)
  (Niagara|SpawnSystematLocation "/Game/HS_Content/FX/FX3_Sparkle.FX3_Sparkle" (Transformation|GetActorLocation))
  (Utilities|Time|SetTimerbyFunctionName 0 "DeathMaterial_sparkle" 0.01 true))

(fn DeathMaterialSparkle
  (CallFunction|TryDeath)
  (bind _output_get (Variables|Default|SetMeterialLevel (- (Variables|Default|GetMeterialLevel) 1.0)))
  (Rendering|Material|SetScalarParameterValue "/Game/HS_Content/Anim/MP_Gloval_Sparkle1_2.MP_Gloval_Sparkle1_2" "Level" _output_get :!class /Script/Engine.KismetMaterialLibrary)
  (if (<= (Variables|Default|GetMeterialLevel) 0.0)
    (Actor|DestroyActor)))