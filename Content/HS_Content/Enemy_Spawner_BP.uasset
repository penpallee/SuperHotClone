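; Enemy spawner actor that, if active, spawns a random enemy at BeginPlay when the checked type is below its cap.
; The spawn point is random within SpawnZone's extent around world origin, not the component.
; A downward trace follows, but its ground snap targets SpawnUnit, which is set to None.
; After a delay it calls an empty SpawnCheck, so nothing repeats; construction sizes both zones, but ShutoffZone has no logic.
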(event Custom|SpawnCheck)

(event EventBeginPlay
  (if (Variables|Default|GetActive?)
    (bind _outactors (Actor|GetAllActorsOfClass (Variables|Default|GetEnemyTypeTo%20Check)))
    (if (>= (Utilities|Array|Length _outactors) (Variables|Default|GetEnemyAmount))
      _
      (else
        (bind _returnvalue (Game|SpawnActorfromClass (.OutItem (Utilities|Array|Random (Variables|Default|GetEnemySpawn))) (Math|Transform|MakeTransform (Math|Random|RandomPointinBoundingBox "0, 0, 0" (Components|Box|GetScaledBoxExtent (Variables|Default|GetSpawnZone))) "0,0.000000, 0" "1.000000,1.000000,1.000000") "Undefined" 0 0))
        (Utilities|IsValid _returnvalue
          (:Is%20Valid
            (bind _output_get (Variables|Default|SetSpawnUnit 0))
            (bind (_outhit _returnvalue_2) (Collision|LineTraceByChannel (Transformation|GetActorLocation _returnvalue) (- (Transformation|GetActorLocation _returnvalue) "0,0,1000.000000") "TraceTypeQuery1" false (Utilities|Array|MakeArray _output_get) "ForDuration"))
            (if _returnvalue_2
              (Transformation|SetActorLocation (Variables|Default|GetSpawnUnit) (+ (.Location (Collision|BreakHitResult _outhit)) "0,0,90.000000") false false)))
          (:Is%20Not%20Valid
            _)))))
  (Utilities|FlowControl|Delay (Variables|Default|GetSpawnDelay))
  (CallFunction|SpawnCheck))

(event Collision|EventActorBeginOverlap
  (params (OtherActor :type Actor%20Object%20Reference)))

(event EventTick
  (params (DeltaSeconds :type Float%20%28single-precision%29)))

(fn ConstructionScript
  (bind _shutoffzone (Variables|Default|GetShutoffZone))
  (Components|Box|SetBoxExtent (Variables|Default|GetSpawnZone) (Variables|Default|GetSpawnZoneSize) true)
  (Components|Box|SetBoxExtent _shutoffzone (Variables|Default|GetShutOffZoneSize) true)
  (Transformation|SetRelativeLocation _shutoffzone (Variables|Default|GetShutOffZoneLocation) false false))