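; Push door Blueprint for the party room that eases toward a fixed angle when the first-person character enters its trigger box.
; The box overlap sets the target angle, and Tick lerps the door mesh's relative rotation toward it using delta time as alpha.
; A hit on the door enables physics simulation, and the scripted rotation stops while the mesh simulates.
; Nothing here closes it again.
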(event OnComponentBeginOverlap(Box)
  (params (OverlappedComponent :type Primitive%20Component%20Object%20Reference) (OtherActor :type Actor%20Object%20Reference) (OtherComp :type Primitive%20Component%20Object%20Reference) (OtherBodyIndex :type Integer) (bFromSweep :type Boolean) (SweepResult :type Hit%20Result%20Structure%20%28by%20ref%29))
  (Utilities|Casting|CastToBP_FirstPersonCharacter OtherActor)
  (Variables|Default|SetTargetAngle "0,20.000000, 0"))

(event OnComponentHit(SM_Door_1)
  (params (HitComponent :type Primitive%20Component%20Object%20Reference) (OtherActor :type Actor%20Object%20Reference) (OtherComp :type Primitive%20Component%20Object%20Reference) (NormalImpulse :type Vector :default "0, 0, 0") (Hit :type Hit%20Result%20Structure%20%28by%20ref%29))
  (Physics|SetSimulatePhysics HitComponent true))

(event EventBeginPlay)

(event Collision|EventActorBeginOverlap
  (params (OtherActor :type Actor%20Object%20Reference)))

(event EventTick
  (params (DeltaSeconds :type Float%20%28single-precision%29))
  (bind _sm_door_1 (Variables|Default|GetSM_Door_1))
  (if (not (Physics|IsSimulatingPhysics (Variables|Default|GetSM_Door_1) "None"))
    (Transformation|SetRelativeRotation _sm_door_1 (Math|Rotator|Lerp(Rotator) (Variables|/Script/Engine.SceneComponent|GetRelativeRotation _sm_door_1) (Variables|Default|GetTargetAngle) DeltaSeconds) false false)))

(fn ConstructionScript)