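; BP_Gun is a pickup gun that fires bullets and can be thrown.
; It caches the player's first-person character on BeginPlay, then Fire spawns a BP_Bullet at its scene point, aimed along that character's camera rotation, and plays the gun animation.
; Collected stops the box's motion and disables its physics and collision, while ThrowGun re-enables both.
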(event EventBeginPlay
  (bind _asbp_first_person_character (Utilities|Casting|CastToBP_FirstPersonCharacter (Game|Player|GetPlayerPawn 0)))
  (Variables|Default|SetPlayer%20ref _asbp_first_person_character))

(event Collision|EventActorBeginOverlap
  (params (OtherActor :type Actor%20Object%20Reference)))

(event EventTick
  (params (DeltaSeconds :type Float%20%28single-precision%29)))

(fn ConstructionScript)

(fn Collected
  (bind _box (Variables|Default|GetBox))
  (Class|PrimitiveComponent|SetAllPhysicsLinearVelocity (Variables|Default|GetBox) "0, 0, 0" false)
  (Physics|SetSimulatePhysics _box false)
  (Collision|SetCollisionEnabled _box "NoCollision"))

(fn Fire
  (Game|SpawnActorfromClass "/Game/Blueprints/BP_Bullet.BP_Bullet_C" (Math|Transform|MakeTransform (Transformation|GetWorldLocation (Variables|Default|GetScene)) (Transformation|GetWorldRotation (Variables|/Game/Blueprints/BP_FirstPersonCharacter.BP_FirstPersonCharacter_C|GetFirstPersonCamera (Variables|Default|GetPlayer%20ref)))) "Undefined" 0 0)
  (Components|Animation|PlayAnimation (Variables|Default|GetTP_Gun) "/Game/StaticMesh/Assets/Meshes/Jericho_941_Anim.Jericho_941_Anim" false))

(fn ThrowGun
  (bind _box (Variables|Default|GetBox))
  (Physics|SetSimulatePhysics _box true)
  (Collision|SetCollisionEnabled _box "QueryAndPhysics"))