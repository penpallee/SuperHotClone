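; Game mode for a SuperHot game that tallies enemies at level start and runs a countdown that pauses the game at zero.
; BeginPlay sets game-only input, shows the alive-enemy widget and sums six punch and gun enemy classes into TotalEnemy.
; HUD initialization shows an intro widget, then enables the timer.
; Tick uses a Delay to decrement Seconds each second, reshowing the start widget on expiry.
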(event EventBeginPlay
  (Input|SetInputModeGameOnly (Game|GetPlayerController 0))
  (bind _returnvalue (UserInterface|CreateWidget "/Game/Blueprints/WBP_AliveEnemy.WBP_AliveEnemy_C"))
  (UserInterface|Viewport|AddtoViewport _returnvalue 0)
  (CallFunction|CountEnemy))

(event EventTick
  (params (DeltaSeconds :type Float%20%28single-precision%29))
  (if (== (Variables|Default|Gettrigger) true)
    (Utilities|FlowControl|Delay 1.0)
    (bind _output_get (Variables|Default|SetSeconds (- (Variables|Default|GetSeconds) 1)))
    (if (== _output_get 0)
      (Game|SetGamePaused true)
      (bind _returnvalue (UserInterface|CreateWidget "/Game/HS_Content/UI/WBP_start.WBP_start_C"))
      (UserInterface|Viewport|AddtoViewport _returnvalue 0))))

(event EventInitializeHUDforPlayer
  (params (NewPlayer :type Player%20Controller%20Object%20Reference))
  (bind _returnvalue (UserInterface|CreateWidget "/Game/HS_Content/UI/WBP_start.WBP_start_C"))
  (UserInterface|Viewport|AddtoViewport _returnvalue 0)
  (Utilities|FlowControl|Delay 6.2)
  (Widget|RemovefromParent _returnvalue)
  (Variables|Default|Settrigger true)
  (bind _returnvalue_2 (UserInterface|CreateWidget "/Game/Blueprints/WBP_Timer.WBP_Timer_C"))
  (UserInterface|Viewport|AddtoViewport _returnvalue_2 0))

(fn ConstructionScript)

(fn CountEnemy
  (bind _outactors (Actor|GetAllActorsOfClass "/Game/HS_Content/BP_Enemy_Punch1.BP_Enemy_Punch1_C"))
  (Variables|Default|SetTotalEnemy (+ (Math|Conversions|ToFloat(Integer) (Utilities|Array|Length _outactors)) (Variables|Default|GetTotalEnemy)))
  (bind _outactors_2 (Actor|GetAllActorsOfClass "/Game/HS_Content/BP_Enemy_Punch1_2.BP_Enemy_Punch1_2_C"))
  (Variables|Default|SetTotalEnemy (+ (Math|Conversions|ToFloat(Integer) (Utilities|Array|Length _outactors_2)) (Variables|Default|GetTotalEnemy)))
  (bind _outactors_3 (Actor|GetAllActorsOfClass "/Game/HS_Content/BP_Enemy_Punch1_3.BP_Enemy_Punch1_3_C"))
  (Variables|Default|SetTotalEnemy (+ (Math|Conversions|ToFloat(Integer) (Utilities|Array|Length _outactors_3)) (Variables|Default|GetTotalEnemy)))
  (bind _outactors_4 (Actor|GetAllActorsOfClass "/Game/HS_Content/BP_Enemy_Gun1.BP_Enemy_Gun1_C"))
  (Variables|Default|SetTotalEnemy (+ (Math|Conversions|ToFloat(Integer) (Utilities|Array|Length _outactors_4)) (Variables|Default|GetTotalEnemy)))
  (bind _outactors_5 (Actor|GetAllActorsOfClass "/Game/HS_Content/BP_Enemy_Gun1_2.BP_Enemy_Gun1_2_C"))
  (Variables|Default|SetTotalEnemy (+ (Utilities|Array|Length _outactors_5) (Variables|Default|GetTotalEnemy)))
  (bind _outactors_6 (Actor|GetAllActorsOfClass "/Game/HS_Content/BP_Enemy_Gun1_3.BP_Enemy_Gun1_3_C"))
  (Variables|Default|SetTotalEnemy (+ (Variables|Default|GetTotalEnemy) (Utilities|Array|Length _outactors_6))))