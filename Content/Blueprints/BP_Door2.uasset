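; BP_Door2 is a door Blueprint that turns on physics simulation and the BlockAll collision profile on its static mesh when another actor begins overlapping it.
; Actor hit and component hit events print their normal impulse to screen, apparently as debug output.
; Tick rebinds the actor hit event every frame and also prints a normal impulse value.
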(event OnComponentHit(StaticMeshComponent)
  (params (HitComponent :type Primitive%20Component%20Object%20Reference) (OtherActor :type Actor%20Object%20Reference) (OtherComp :type Primitive%20Component%20Object%20Reference) (NormalImpulse :type Vector :default "0, 0, 0") (Hit :type Hit%20Result%20Structure%20%28by%20ref%29))
  (Development|PrintString (Utilities|String|ToString(Vector) NormalImpulse)))

(event Custom|OnActorHit_Event
  (params (SelfActor :type Actor%20Object%20Reference) (OtherActor :type Actor%20Object%20Reference) (NormalImpulse :type Vector) (Hit :type Hit%20Result%20Structure%20%28by%20ref%29))
  (Development|PrintString (Utilities|String|ToString(Vector) NormalImpulse)))

(event EventBeginPlay)

(event Collision|EventActorBeginOverlap
  (params (OtherActor :type Actor%20Object%20Reference))
  (Physics|SetSimulatePhysics (Variables|Debug|GetStaticMeshComponent) true)
  (Collision|SetCollisionProfileName (Variables|Debug|GetStaticMeshComponent) "BlockAll" true :!class /Script/Engine.PrimitiveComponent))

(event EventTick
  (params (DeltaSeconds :type Float%20%28single-precision%29))
  (EventDispatchers|BindEventtoOnActorHit (delegate Custom|OnActorHit_Event))
  (Development|PrintString (Utilities|String|ToString(Vector) (stale Custom|OnActorHit_Event NormalImpulse))))

(fn ConstructionScript)