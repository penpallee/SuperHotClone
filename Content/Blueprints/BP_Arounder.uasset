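; BP_Arounder is an actor Blueprint that drives its own position with a time-based sine wave.
; Tick accumulates RunningTime and feeds it to AroundMove as AroundSpeed.
; AroundMove sets an absolute location, deriving Z from the scaled sine difference over one frame, without adding the current position.
; Its Direction input is unused, and a direction-based movement calculation is left disconnected.
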(event EventBeginPlay)

(event Collision|EventActorBeginOverlap
  (params (OtherActor :type Actor%20Object%20Reference)))

(event EventTick
  (params (DeltaSeconds :type Float%20%28single-precision%29))
  (bind _output_get (Variables|Default|SetRunningTime (+ (Utilities|Time|GetWorldDeltaSeconds) (Variables|Default|GetRunningTime))))
  (CallFunction|AroundMove "0, 0, 0" _output_get))

(fn ConstructionScript)

(fn AroundMove
  (params (Direction :type Vector) (AroundSpeed :type Float%20%28double-precision%29))
  (Transformation|SetActorLocation (Math|Vector|MakeVector 0.0 0.0 (* 2e+01 (- (Math|Trig|Sin(Radians) (+ AroundSpeed (Utilities|Time|GetWorldDeltaSeconds))) (Math|Trig|Sin(Radians) AroundSpeed)))) false false))